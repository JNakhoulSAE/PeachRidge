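; BP_PhoneV2 is the player's phone, used to photograph and scan species.
; Each tick it sits just in front of the player pawn, matching its rotation.
; PhotoTaken flashes a white camera fade, then matches queued SpeciesToScan display names against GM_Main's scannable list by substring, recording matches in ScannedSpecies.
; Valid queued entries then have their billboard sprite cleared and leave the player's queue, which also empties at BeginPlay.
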(event Custom|Photo%20Taken
  (bind _returnvalue (Game|GetGameMode))
  (bind _returnvalue_2 (Game|Player|GetPlayerPawn 0))
  (bind _asgm_main (Utilities|Casting|CastToGM_Main _returnvalue))
  (bind _aschr_player (Utilities|Casting|CastToCHR_Player _returnvalue_2))
  (bind _speciestoscan (Variables|/Game/MobileControllers/CHR_Player.CHR_Player_C|GetspeciesToScan _aschr_player))
  (CameraFades|StartCameraFade (Game|GetPlayerCameraManager 0) 0.5 0.0 0.5 "(R=1.000000,G=1.000000,B=1.000000,A=1.000000)" false true)
  (for _index (range 0 2)
    (if (Utilities|Array|IsValidIndex _speciestoscan _index)
      (Variables|Default|SetcanStartScanning true)))
  (if (Variables|Default|GetcanStartScanning)
    (for _array_element _speciestoscan
      (Utilities|IsValid _array_element
        (:Is%20Valid
          ;[1 1 1] Adding species to list of all scanned species
          (bind _array_element_2 (Utilities|Array|ForEachLoopwithBreak (Variables|/Game/Blueprints/GM_Main.GM_Main_C|GetscannableSpecies _asgm_main))
            (:LoopBody
              (if (Utilities|String|Contains (Utilities|GetDisplayName _array_element) _array_element_2)
                (Development|PrintString (Utilities|String|Append "Scanned " _array_element_2) true true "(R=0.785505,G=0.000000,B=1.000000,A=1.000000)")
                (Utilities|Array|AddUnique (Variables|/Game/Blueprints/GM_Main.GM_Main_C|GetscannedSpecies _asgm_main) _array_element_2)))
            (:Completed
              (Rendering|Components|Sprite|SetSprite (Actor|GetComponentbyClass _array_element "/Script/Engine.BillboardComponent") 0)
              (Utilities|Array|RemoveItem _speciestoscan _array_element))))))
    (Variables|Default|SetcanStartScanning false)
    (else
      (Development|PrintString "No species to scan.")
      (Variables|Default|SetcanStartScanning false))))

(event EventTick
  (params (DeltaSeconds :type Float%20%28single-precision%29))
  (bind _returnvalue (Game|Player|GetPlayerPawn 0))
  (bind _returnvalue_2 (Transformation|GetActorTransform _returnvalue))
  (Transformation|SetActorLocationAndRotation (+ (* (Transformation|GetActorForwardVector _returnvalue) 100) (.location _returnvalue_2)) (.rotation _returnvalue_2)))

(event EventBeginPlay
  (Utilities|Array|Clear (Variables|/Game/MobileControllers/CHR_Player.CHR_Player_C|GetspeciesToScan (.AsCHR%20Player (Utilities|Casting|CastToCHR_Player (Game|Player|GetPlayerPawn 0))))))

(fn ConstructionScript)