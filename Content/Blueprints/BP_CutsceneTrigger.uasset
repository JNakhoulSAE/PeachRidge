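; Trigger volume Blueprint that plays the Archway MP4 cutscene through a media player, opened on BeginPlay.
; The first overlap of any actor consumes a DoOnce, then continues only if that actor's display name contains "player".
; It fades to black, shows a UI_Cutscene widget, starts playback and moves the actor to a hardcoded location.
; A fixed delay, rather than a media-end event, times widget removal and fade back in.
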(event OnComponentBeginOverlap(TriggerBox)
  (params (OverlappedComponent :type Primitive%20Component%20Object%20Reference) (OtherActor :type Actor%20Object%20Reference) (OtherComp :type Primitive%20Component%20Object%20Reference) (OtherBodyIndex :type Integer) (bFromSweep :type Boolean) (SweepResult :type Hit%20Result%20Structure%20%28by%20ref%29))
  (Utilities|FlowControl|DoOnce false
    (:Completed
      (if (Utilities|String|Contains (Utilities|GetDisplayName OtherActor) "player")
        (CallFunction|Fadein)
        (Utilities|FlowControl|Delay 0.5)
        (bind _returnvalue (UserInterface|CreateWidget "/Game/Blueprints/UI/CutScene/UI_Cutscene.UI_Cutscene_C" (Game|GetPlayerController 0)))
        (UserInterface|Viewport|AddtoViewport _returnvalue 0)
        (Media|MediaPlayer|Play (Variables|Default|GetmediaPlayer) :!class /Script/MediaAssets.MediaPlayer)
        (Transformation|SetActorLocation OtherActor "-100.000000,200.000000,770.000000" false false)
        (Utilities|FlowControl|Delay 9.5)
        (Widget|RemovefromParent _returnvalue)
        (CallFunction|FadeOut)))))

(event EventBeginPlay
  (Media|MediaPlayer|OpenSource (Variables|Default|GetmediaPlayer) "/Game/Video/CutScene/Archway/MP4_CTSCN_Archway.MP4_CTSCN_Archway"))

(fn ConstructionScript)

(fn Fadein
  (CameraFades|StartCameraFade (Game|GetPlayerCameraManager 0) 0.0 1.0 0.5 "(R=0.000000,G=0.000000,B=0.000000,A=1.000000)" false true))

(fn FadeOut
  (CameraFades|StartCameraFade (Game|GetPlayerCameraManager 0) 1.0 0.0 1.0 "(R=0.000000,G=0.000000,B=0.000000,A=1.000000)" false true))