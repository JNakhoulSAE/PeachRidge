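; Giant cod actor Blueprint that swims along a referenced spline track when FishActive is set at BeginPlay.
; A timeline starts from FishStartPosition, with its play rate set to the inverse of Duration to control swim time.
; Each update maps the timeline alpha to a distance along the spline and applies that point's world location and rotation to the fish.
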(event Custom|FishSwim
  ;[1 1 1] Set Time & Duration of Fish Movement
  (Components|Timeline|SetNewTime (Variables|Default|GetMoveFish_TimeLine) (Variables|Default|GetFishStartPosition))
  (Components|Timeline|SetPlayRate (Variables|Default|GetMoveFish_TimeLine) (/ 1.0 (Variables|Default|GetDuration)))
  (bind _alpha_time_ (Timeline|MoveFish_TimeLine Play)
    (:Update
      (Variables|Default|SetAlpha%28Time%29 _alpha_time_)
      ;[1 1 1] Set Current Location & Rotation of Fish Along Spline
      (Transformation|SetActorLocationAndRotation (Spline|GetLocationatDistanceAlongSpline (Variables|/Game/Blueprints/SplineTest/BP_F_SplineTrack_Master.BP_F_SplineTrack_Master_C|GetF_SplineTrack (Variables|Default|GetSplineTrack)) (Math|Float|Lerp 0.0 (Spline|GetSplineLength (Variables|/Game/Blueprints/SplineTest/BP_F_SplineTrack_Master.BP_F_SplineTrack_Master_C|GetF_SplineTrack (Variables|Default|GetSplineTrack))) (Variables|Default|GetAlpha%28Time%29)) "World") (Spline|GetRotationatDistanceAlongSpline (Variables|/Game/Blueprints/SplineTest/BP_F_SplineTrack_Master.BP_F_SplineTrack_Master_C|GetF_SplineTrack (Variables|Default|GetSplineTrack)) (Math|Float|Lerp 0.0 (Spline|GetSplineLength (Variables|/Game/Blueprints/SplineTest/BP_F_SplineTrack_Master.BP_F_SplineTrack_Master_C|GetF_SplineTrack (Variables|Default|GetSplineTrack))) (Variables|Default|GetAlpha%28Time%29)) "World")))))

(event EventBeginPlay
  ;[1 1 1] Play Fish Movement
  (if (Variables|Default|GetFishActive)
    (CallFunction|FishSwim)))

(fn ConstructionScript)