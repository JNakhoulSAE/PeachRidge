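; Master Blueprint for a beer bottle trash item that brings up a trash selection UI when the player comes near.
; On BeginPlay, after a short delay, it reuses an existing top-level UI_TrashSelect widget or creates one and adds it to the viewport.
; Sphere overlap by an actor whose display name contains "player" assigns this bottle to the widget and makes it visible.
; The file has no logic to hide the widget again.
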(event OnComponentBeginOverlap(Sphere)
  (params (OverlappedComponent :type Primitive%20Component%20Object%20Reference) (OtherActor :type Actor%20Object%20Reference) (OtherComp :type Primitive%20Component%20Object%20Reference) (OtherBodyIndex :type Integer) (bFromSweep :type Boolean) (SweepResult :type Hit%20Result%20Structure%20%28by%20ref%29))
  (bind __trashselectwidget (Variables|Default|Get_trashSelectWidget))
  (if (Utilities|String|Contains (Utilities|GetDisplayName OtherActor) "player")
    (Variables|/Game/Blueprints/UI/UI_TrashSelect.UI_TrashSelect_C|Settrash __trashselectwidget self)
    (Widget|SetVisibility __trashselectwidget "Visible")))

(event EventBeginPlay
  (Utilities|FlowControl|Delay 0.1)
  (bind _foundwidgets (Widget|GetAllWidgetsOfClass "/Game/Blueprints/UI/UI_TrashSelect.UI_TrashSelect_C" true))
  (if (Utilities|Array|IsValidIndex _foundwidgets)
    (Variables|Default|Set_trashSelectWidget (Utilities|Array|Get(acopy) _foundwidgets))
    (else
      (bind _returnvalue (UserInterface|CreateWidget "/Game/Blueprints/UI/UI_TrashSelect.UI_TrashSelect_C" (Game|GetPlayerController 0)))
      (bind _output_get (Variables|Default|Set_trashSelectWidget _returnvalue))
      (UserInterface|Viewport|AddtoViewport _output_get 0))))

(fn ConstructionScript)