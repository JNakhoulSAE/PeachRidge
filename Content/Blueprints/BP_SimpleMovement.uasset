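; BP_SimpleMovement is an actor that roams endlessly between randomly chosen TargetPoints in the level.
; BeginPlay gathers the TargetPoints, picks one and turns the actor toward it.
; Tick, throttled by a short Delay, steps it forward by Speed without sweep or delta-time scaling, re-picking and re-aiming on arrival.
; Nested random calls bias selection toward lower array indices and can repeat the current target.
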(event EventBeginPlay
  (bind _outactors (Actor|GetAllActorsOfClass "/Script/Engine.TargetPoint"))
  (bind _output_get (Variables|Default|Setcheckpoints _outactors))
  (bind _output_get_2 (Variables|Default|SetcurrentTarget (Utilities|Array|Get(acopy) _output_get (Math|Random|RandomInteger (+ (Math|Random|RandomInteger (Utilities|Array|Length (Variables|Default|Getcheckpoints))) 1)))))
  (Transformation|SetActorRotation (Math|Rotator|FindLookatRotation (Transformation|GetActorLocation) (Transformation|GetActorLocation _output_get_2))))

(event EventTick
  (params (DeltaSeconds :type Float%20%28single-precision%29))
  (bind _checkpoints (Variables|Default|Getcheckpoints))
  (Utilities|FlowControl|Delay 0.01)
  (Transformation|SetActorLocation (+ (Transformation|GetActorLocation) (* (Transformation|GetActorForwardVector) (Variables|Default|Getspeed))) false false)
  (if (Math|Vector|Equal(Vector) (Transformation|GetActorLocation) (Transformation|GetActorLocation (Variables|Default|GetcurrentTarget)) 1e+01)
    (bind _output_get (Variables|Default|SetcurrentTarget (Utilities|Array|Get(acopy) _checkpoints (Math|Random|RandomInteger (+ (Math|Random|RandomInteger (Utilities|Array|Length _checkpoints)) 1)))))
    (Transformation|SetActorRotation (Math|Rotator|FindLookatRotation (Transformation|GetActorLocation) (Transformation|GetActorLocation _output_get)))))

(fn ConstructionScript)