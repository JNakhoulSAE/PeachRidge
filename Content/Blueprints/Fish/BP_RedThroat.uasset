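; BP_RedThroat is a fish that swims between TargetPoint checkpoints in its own district.
; On BeginPlay it collects TargetPoints tagged with its DistrictID, picks one through a nested random index that favors earlier entries, and snaps to face it.
; A timeline nudges it along its forward vector, scaled by Speed, on each update.
; When it comes close to the target, it picks again, looping back into the same selection.
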(event EventBeginPlay
  (bind _returnvalue (Transformation|GetActorLocation))
  (bind _checkpoints (Variables|Default|Getcheckpoints))
  ;[1 1 1] Set fish checkpoints
  (bind _outactors (Actor|GetAllActorsOfClass "/Script/Engine.TargetPoint"))
  (for _array_element _outactors
    (if (Actor|ActorHasTag _array_element (Variables|Default|GetdistrictID))
      (Utilities|Array|Add (Variables|Default|Getcheckpoints) _array_element)))
  ;[1 1 1] Choose new checkpoint
  (bind _output_get (Variables|Default|SetcurrentTarget (Utilities|Array|Get(acopy) _checkpoints (Math|Random|RandomInteger (+ (Math|Random|RandomInteger (Utilities|Array|Length _checkpoints)) 1))) :!label _label))
  (Transformation|SetActorRotation (Math|Rotator|FindLookatRotation (Transformation|GetActorLocation) (Transformation|GetActorLocation _output_get)))
  ;[1 1 1] Move Forwards
  (bind _lerpedalpha (Timeline|Timeline_0 Play)
    (:Update
      (Transformation|SetActorLocation (Math|Vector|Lerp(Vector) _returnvalue (+ _returnvalue (* (Transformation|GetActorForwardVector) (Variables|Default|Getspeed))) _lerpedalpha) false false)
      ;[1 1 1] Has fish has reached it's current target?
      (if (Math|Vector|Equal(Vector) (Transformation|GetActorLocation) (Transformation|GetActorLocation (Variables|Default|GetcurrentTarget)) 1e+01)
        (goto _label)))))

(fn ConstructionScript)