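; Giant clam animation trigger that reacts to the player entering and leaving a box volume.
; Begin overlap plays the Animation variable once on the skeletal mesh.
; End overlap calls PlayAnimation without that variable, then sets the play rate to -1 for reverse playback; begin overlap never resets the rate.
; Both events identify the player by searching the overlapping actor's display name for "player".
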(event OnComponentBeginOverlap(Box)
  (params (OverlappedComponent :type Primitive%20Component%20Object%20Reference) (OtherActor :type Actor%20Object%20Reference) (OtherComp :type Primitive%20Component%20Object%20Reference) (OtherBodyIndex :type Integer) (bFromSweep :type Boolean) (SweepResult :type Hit%20Result%20Structure%20%28by%20ref%29))
  (if (Utilities|String|Contains (Utilities|GetDisplayName OtherActor) "player")
    (Components|Animation|PlayAnimation (Variables|Default|GetSkeletalMesh) (Variables|Default|Getanimation) false)))

(event OnComponentEndOverlap(Box)
  (params (OverlappedComponent :type Primitive%20Component%20Object%20Reference) (OtherActor :type Actor%20Object%20Reference) (OtherComp :type Primitive%20Component%20Object%20Reference) (OtherBodyIndex :type Integer))
  (bind _skeletalmesh (Variables|Default|GetSkeletalMesh))
  (if (Utilities|String|Contains (Utilities|GetDisplayName OtherActor) "player")
    (Components|Animation|PlayAnimation _skeletalmesh 0 false)
    (Components|Timeline|SetPlayRate _skeletalmesh -1.0)))

(fn ConstructionScript)