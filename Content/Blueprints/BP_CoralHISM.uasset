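; BP_CoralHISM places many kinds of coral as instanced meshes, with a separate hierarchical instanced static mesh component for each species or variant.
; The construction script loops over a location array for each type, from tube, elkhorn and staghorn to seapen and bubble, and adds each entry as an instance to its matching component.
; The event graph has no active logic.
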(event EventBeginPlay)

(event Collision|EventActorBeginOverlap
  (params (OtherActor :type Actor%20Object%20Reference)))

(event EventTick
  (params (DeltaSeconds :type Float%20%28single-precision%29)))

(fn ConstructionScript
  (for _array_element (Variables|LocationArrays|GettubeCoralA_Locations)
    (Components|InstancedStaticMesh|AddInstance (Variables|Default|GetHISM_TubeA) _array_element))
  (for _array_element_2 (Variables|LocationArrays|GettubeCoralB_Locations)
    (Components|InstancedStaticMesh|AddInstance (Variables|Default|GetHISM_TubeB) _array_element_2))
  (for _array_element_3 (Variables|LocationArrays|GetelkhornA_locations)
    (Components|InstancedStaticMesh|AddInstance (Variables|Default|GetHISM_ElkhornA) _array_element_3))
  (for _array_element_4 (Variables|LocationArrays|GetelkhornB_Locations)
    (Components|InstancedStaticMesh|AddInstance (Variables|Default|GetHISM_ElkhornB) _array_element_4))
  (for _array_element_5 (Variables|LocationArrays|GetstaghornA_Locations)
    (Components|InstancedStaticMesh|AddInstance (Variables|Default|GetHISM_StaghornA) _array_element_5))
  (for _array_element_6 (Variables|LocationArrays|GetstaghornB_Locations)
    (Components|InstancedStaticMesh|AddInstance (Variables|Default|GetHISM_StaghornB) _array_element_6))
  (for _array_element_7 (Variables|LocationArrays|GetcarnationA_Locations)
    (Components|InstancedStaticMesh|AddInstance (Variables|Default|GetHISM_CarnationA) _array_element_7))
  (for _array_element_8 (Variables|LocationArrays|GetcarnationB_Locations)
    (Components|InstancedStaticMesh|AddInstance (Variables|Default|GetHISM_CarnationB) _array_element_8))
  (for _array_element_9 (Variables|LocationArrays|GetgeorgianA_Locations)
    (Components|InstancedStaticMesh|AddInstance (Variables|Default|GetHISM_GeorgianA) _array_element_9))
  (for _array_element_10 (Variables|LocationArrays|GetgeorgianB_Locations)
    (Components|InstancedStaticMesh|AddInstance (Variables|Default|GetHISM_GeorgianB) _array_element_10))
  (for _array_element_11 (Variables|LocationArrays|GetblueCoral_Locations)
    (Components|InstancedStaticMesh|AddInstance (Variables|Default|GetHISM_Blue) _array_element_11))
  (for _array_element_12 (Variables|LocationArrays|GetbrainCoral_Locations)
    (Components|InstancedStaticMesh|AddInstance (Variables|Default|GetHISM_Brain) _array_element_12))
  (for _array_element_13 (Variables|LocationArrays|GetpillarCoral_Locations)
    (Components|InstancedStaticMesh|AddInstance (Variables|Default|GetHISM_Pillar) _array_element_13))
  (for _array_element_14 (Variables|LocationArrays|GettableCoralA_Locations)
    (Components|InstancedStaticMesh|AddInstance (Variables|Default|GetHISM_TableA) _array_element_14))
  (for _array_element_15 (Variables|LocationArrays|GettableCoralB_Locations)
    (Components|InstancedStaticMesh|AddInstance (Variables|Default|GetHISM_TableB) _array_element_15))
  (for _array_element_16 (Variables|LocationArrays|GettoadstoolA_Locations)
    (Components|InstancedStaticMesh|AddInstance (Variables|Default|GetHISM_ToadstoolA) _array_element_16))
  (for _array_element_17 (Variables|LocationArrays|GettoadstoolB_Locations)
    (Components|InstancedStaticMesh|AddInstance (Variables|Default|GetHISM_ToadstoolB) _array_element_17))
  (for _array_element_18 (Variables|LocationArrays|Getseapen_Locations)
    (Components|InstancedStaticMesh|AddInstance (Variables|Default|GetHISM_Seapen) _array_element_18))
  (for _array_element_19 (Variables|LocationArrays|Getbubble_Locations)
    (Components|InstancedStaticMesh|AddInstance (Variables|Default|GetHISM_Bubble) _array_element_19)))