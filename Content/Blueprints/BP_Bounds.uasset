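; Bounds actor that triggers the end-dive screen when the player leaves its bounding box during a dive.
; End overlap on a player-named actor, or pressing F, stores the exit position, switches GM_Main's controller mode, fades to black, enables UI_EndDive and stops player movement.
; ReturnToDive moves the pawn back to the stored position; a look-at rotation toward the "Center"-tagged actor is left unused.
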(event OnComponentEndOverlap(BoundingBox)
  (params (OverlappedComponent :type Primitive%20Component%20Object%20Reference) (OtherActor :type Actor%20Object%20Reference) (OtherComp :type Primitive%20Component%20Object%20Reference) (OtherBodyIndex :type Integer))
  (if (Utilities|String|Contains (Utilities|GetDisplayName OtherActor) "player")
    (Variables|Default|SetexitPos (Transformation|GetActorLocation OtherActor))
    ;[1 1 1] Start out of bounds screen
    (Variables|/Game/Blueprints/GM_Main.GM_Main_C|SetcurrentControllerMode (.AsGM%20Main (Utilities|Casting|CastToGM_Main (Game|GetGameMode))) "NewEnumerator2")
    (CameraFades|StartCameraFade (Game|GetPlayerCameraManager 0) 0.0 1.0 0.5 "(R=0.000000,G=0.000000,B=0.000000,A=1.000000)" false true)
    (Variables|/Game/Blueprints/UI/UI_EndDive.UI_EndDive_C|SetisEnabled (stale EventBeginPlay _returnvalue) true)
    (Variables|/Game/MobileControllers/CHR_Player.CHR_Player_C|Setmoving (.AsCHR%20Player (Utilities|Casting|CastToCHR_Player (Game|Player|GetPlayerPawn 0))) false)))

(event Custom|ReturnToDive
  (bind _outactors (Actor|GetAllActorswithTag "Center"))
  (Transformation|SetActorLocationAndRotation (Game|Player|GetPlayerPawn 0) (Variables|Default|GetexitPos)))

(event EventBeginPlay
  (Input|EnableInput (Game|GetPlayerController 0))
  (bind _returnvalue (UserInterface|CreateWidget "/Game/Blueprints/UI/UI_EndDive.UI_EndDive_C" (Game|GetPlayerController 0)))
  (UserInterface|Viewport|AddtoViewport _returnvalue 0)
  (Variables|/Game/Blueprints/UI/UI_EndDive.UI_EndDive_C|SetisEnabled _returnvalue false))

(event Input|KeyboardEvents|F
  (params (Key :type Key%20Structure))
  (:Pressed
    (Variables|Default|SetexitPos (Transformation|GetActorLocation (stale OnComponentEndOverlap(BoundingBox) OtherActor)))
    ;[1 1 1] Start out of bounds screen
    (Variables|/Game/Blueprints/GM_Main.GM_Main_C|SetcurrentControllerMode (.AsGM%20Main (Utilities|Casting|CastToGM_Main (Game|GetGameMode))) "NewEnumerator2")
    (CameraFades|StartCameraFade (Game|GetPlayerCameraManager 0) 0.0 1.0 0.5 "(R=0.000000,G=0.000000,B=0.000000,A=1.000000)" false true)
    (Variables|/Game/Blueprints/UI/UI_EndDive.UI_EndDive_C|SetisEnabled (stale EventBeginPlay _returnvalue) true)
    (Variables|/Game/MobileControllers/CHR_Player.CHR_Player_C|Setmoving (.AsCHR%20Player (Utilities|Casting|CastToCHR_Player (Game|Player|GetPlayerPawn 0))) false)))

(fn ConstructionScript)